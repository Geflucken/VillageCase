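; Game mode for a murder mystery that randomly casts a murderer and a different victim from the Villagers data table.
; On BeginPlay it teleports the victim, found by occupation tag, to a random spot and plays a death animation.
; The player's found-item event is checked against a CurrentTarget tag, advancing a state counter through body, weapon and murderer.
; Event dispatchers chain stages: finding the body spawns an axe at the murderer's house, finding it targets the murderer.
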(event `self.ReceiveBeginPlay`
  (set `self.StateNumber` -1)
  (add `self.FoundBody` (delegate `HandleFoundBody`))
  (add `self.FoundWeapon` (delegate `HandleFoundWeapon`))
  (`self.RandomizeMurderCase`)
  ;[1 1 1] Make sure Murderer is not the Victim too
  (while (`KismetStringLibrary.EqualEqual_StrStr` (`.Occupation_3_D98A1F284AC7167EBE0414A16EEF195D` (break `/Game/GameModes/Villager` (`self.Murderer`))) (`.Occupation_3_D98A1F284AC7167EBE0414A16EEF195D` (break `/Game/GameModes/Villager` (`self.Victim`))))
    (`self.RandomizeMurderCase`))
  (bind _output_get (set `self.CurrentTarget` (`KismetStringLibrary.Conv_StringToName` (`.Occupation_3_D98A1F284AC7167EBE0414A16EEF195D` (break `/Game/GameModes/Villager` (`self.Victim`))))))
  (bind _outactors (`GameplayStatics.GetAllActorsWithTag` _output_get))
  (for _array_element _outactors
    (bind _asue_4asp_character (cast `/Game/NPC/Character/Ue4ASP_Character` _array_element))
    (`self.K2_SetActorLocation` _asue_4asp_character (`KismetMathLibrary.RandomPointInBoundingBox` (9000.0 2100.0 200.0) (1000.0 1000.0 0.0)) false true)
    (bind _mesh (`Character.Mesh` _asue_4asp_character))
    (`SkeletalMeshComponent.SetAnimationMode` _mesh "AnimationSingleNode")
    (`SkeletalMeshComponent.PlayAnimation` _mesh "/Game/NPC/Animations/Death_1.Death_1" false))
  (bind _asbp_first_person_player (cast `/Game/Player/Behaviour/BP_FirstPersonPlayer` (`GameplayStatics.GetPlayerCharacter` 0)))
  (add `/Game/Player/Behaviour/BP_FirstPersonPlayer.FoundItem` _asbp_first_person_player (delegate `CheckItemFound`)))

(event `HandleFoundBody`
  (`self.SpawnWeapon`))

(event `HandleFoundWeapon`
  (`self.DetermineMurderer`))

(event `CheckItemFound`
  (params (ItemTags :type "Array of Name (by ref)"))
  ;[1 1 1] Check if the Player clicks the Current Target
  (if (`KismetArrayLibrary.Array_Contains` ItemTags (`self.CurrentTarget`))
    (bind _result (`/Engine/EditorBlueprintResources/StandardMacros.IncrementInt` (`self.StateNumber`))
      (:`  `
        (switch `int` _result
          (:`0`
            (`self.FoundBody`))
          (:`1`
            (`self.FoundWeapon`))
          (:`2`
            (`self.FoundMurderer`)))))))

(event `SpawnWeapon`
  ;[1 1 1] Spawn Weapon in the house of the murderer
  (bind _returnvalue (`|SpawnActorFromClass` "/Game/GameModes/BP_Spawner.BP_Spawner_C" (`KismetMathLibrary.Conv_VectorToTransform` (`.HouseLocation_11_6D2949FF4533C883AA749D8655AA15D2` (break `/Game/GameModes/Villager` (`self.Murderer`)))) "AdjustIfPossibleButAlwaysSpawn" "OverrideRootScale" null null))
  (`Spawner.PlaceActor` _returnvalue "/Game/Custom/Blueprints/BP_Axe.BP_Axe_C" 100.0)
  (set `self.CurrentTarget` "MurderWeapon")
  (remove `self.FoundBody` (delegate `HandleFoundBody`)))

(event `DetermineMurderer`
  ;[1 1 1] Set Murderer as Target
  (set `self.CurrentTarget` (`KismetStringLibrary.Conv_StringToName` (`.Occupation_3_D98A1F284AC7167EBE0414A16EEF195D` (break `/Game/GameModes/Villager` (`self.Murderer`)))))
  (remove `self.FoundWeapon` (delegate `HandleFoundWeapon`)))

(fn `RandomizeMurderCase`
  (locals (RandomStream :type "RandomStream Structure"))
  (bind _returnvalue (`|GetDataTableRow` "/Game/GameModes/Villagers.Villagers" (`KismetStringLibrary.Conv_StringToName` (`KismetStringLibrary.Conv_IntToString` (`KismetMathLibrary.RandomIntegerInRange` 1 3))))
    (:`then`
      (set `self.Murderer` _returnvalue)
      (bind _returnvalue_2 (`|GetDataTableRow` "/Game/GameModes/Villagers.Villagers" (`KismetStringLibrary.Conv_StringToName` (`KismetStringLibrary.Conv_IntToString` (`KismetMathLibrary.RandomIntegerInRange` 1 3))))
        (:`then`
          (set `self.Victim` _returnvalue_2))))))

(fn `UserConstructionScript`
  (`parent.UserConstructionScript`))