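; Blacksmith NPC for the Murder game mode that opens a dialogue when clicked and gives a clue to the murderer.
; Conversation 0 uses the parent's dialogue; later ones fill a new DialogueUI widget from DialogueGetLine.
; The second answer gets the murderer's occupation appended from BP_Murder_GameMode.
; Opening this dialogue switches input to UI-only with a cursor and immediately tells the game mode to spawn the weapon.
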(event `self.Clicked`
  (`self.SetDialogue`)
  (if (== (`self.Conversation_ID`) 1)
    _))

(event `self.SetDialogue`
  (bind _returnvalue (`GameplayStatics.GetPlayerController` 0))
  (bind _dialogueui (`self.DialogueUI`))
  (if (== (`self.Conversation_ID`) 0)
    (`parent.SetDialogue`)
    (else
      (bind _returnvalue_2 (`|CreateWidget` "/Game/Player/UI/DialogueUI.DialogueUI_C"))
      (bind _output_get (set `self.DialogueUI` _returnvalue_2))
      (bind (_question1 _answer1 _question2 _answer2 _greet _bye) (`self.DialogueGetLine`))
      (set `/Game/Player/UI/DialogueUI.Dialogue1` _question1 _dialogueui)
      (set `/Game/Player/UI/DialogueUI.Answer1` _answer1 _dialogueui)
      (set `/Game/Player/UI/DialogueUI.Dialogue2` _question2 _dialogueui)
      (bind _asbp_murder_game_mode (cast `/Game/GameModes/Murder/BP_Murder_GameMode` (`GameplayStatics.GetGameMode`)))
      (set `/Game/Player/UI/DialogueUI.Answer2` (`KismetTextLibrary.Conv_StringToText` (`KismetStringLibrary.Concat_StrStr` (`KismetTextLibrary.Conv_TextToString` _answer2) " " (`.Occupation_3_D98A1F284AC7167EBE0414A16EEF195D` (break `/Game/GameModes/Villager` (`/Game/GameModes/Murder/BP_Murder_GameMode.MurdererStruct` _asbp_murder_game_mode))))) _dialogueui)
      (set `/Game/Player/UI/DialogueUI.Greet` _greet _dialogueui)
      (set `/Game/Player/UI/DialogueUI.Dialogue3` _bye _dialogueui)
      (`UserWidget.AddToViewport` _output_get 0)
      (`WidgetBlueprintLibrary.SetInputMode_UIOnlyEx` _returnvalue _returnvalue_2)
      (set `PlayerController.bShowMouseCursor` true _returnvalue)
      (`/Game/GameModes/Murder/BP_Murder_GameMode.SpawnWeapon` _asbp_murder_game_mode))))

(fn `UserConstructionScript`
  (`parent.UserConstructionScript`))